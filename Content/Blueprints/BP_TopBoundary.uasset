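; BP_TopBoundary is a box volume that acts as a water surface limit for the player character.
; On overlap begin, it disables the player's CanMove, switches movement to Falling, plays a splash-out sound and clears the bubble timer.
; On overlap end, it restores CanMove, switches to Flying as the underwater movement mode, plays a splash-in sound and restarts the bubble trail.
; It responds only to the BP_ThirdPersonCharacter cached at BeginPlay.
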(event OnComponentBeginOverlap(Box)
  (params (OverlappedComponent :type Primitive%20Component%20Object%20Reference) (OtherActor :type Actor%20Object%20Reference) (OtherComp :type Primitive%20Component%20Object%20Reference) (OtherBodyIndex :type Integer) (bFromSweep :type Boolean) (SweepResult :type Hit%20Result%20Structure%20%28by%20ref%29))
  (bind _playerref (Variables|Default|GetPlayerRef))
  (if (== OtherActor _playerref)
    (Variables|/Game/ThirdPerson/Blueprints/BP_ThirdPersonCharacter.BP_ThirdPersonCharacter_C|SetCanMove _playerref false)
    (Pawn|Components|CharacterMovement|SetMovementMode (Variables|/Script/Engine.Character|GetCharacterMovement _playerref) "MOVE_Falling" 0)
    (Audio|PlaySound2D "/Game/SFX/SFX_SplashOut.SFX_SplashOut" 1.0 1.0 0.0 0 0)
    (Utilities|Time|ClearandInvalidateTimerbyHandle (Variables|/Game/ThirdPerson/Blueprints/BP_ThirdPersonCharacter.BP_ThirdPersonCharacter_C|GetBubbleTimer (Variables|Default|GetPlayerRef)))))

(event OnComponentEndOverlap(Box)
  (params (OverlappedComponent :type Primitive%20Component%20Object%20Reference) (OtherActor :type Actor%20Object%20Reference) (OtherComp :type Primitive%20Component%20Object%20Reference) (OtherBodyIndex :type Integer))
  (bind _playerref (Variables|Default|GetPlayerRef))
  (if (== OtherActor _playerref)
    (Variables|/Game/ThirdPerson/Blueprints/BP_ThirdPersonCharacter.BP_ThirdPersonCharacter_C|SetCanMove _playerref true)
    (Pawn|Components|CharacterMovement|SetMovementMode (Variables|/Script/Engine.Character|GetCharacterMovement _playerref) "MOVE_Flying" 0)
    (Audio|PlaySound2D "/Game/SFX/SFX_SplashIn.SFX_SplashIn" 1.0 1.0 0.0 0 0)
    (Default|StartBubbleTrail (Variables|Default|GetPlayerRef))))

(event EventBeginPlay
  (bind _asbp_third_person_character (Utilities|Casting|CastToBP_ThirdPersonCharacter (Game|Player|GetPlayerPawn 0)))
  (Variables|Default|SetPlayerRef _asbp_third_person_character))

(fn ConstructionScript)