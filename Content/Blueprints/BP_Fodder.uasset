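; BP_Fodder is a bobbing coral pickup that the player consumes when larger than it, either growing or losing health.
; On BeginPlay it rolls a level-scaled size and a chance to be an enemy, coloring its dynamic materials to match.
; Interact damages the player for enemies, otherwise grows player, camera boom and attached coral, then destroys the fodder.
; The player's OnCoralConsumed dispatcher triggers each fodder's edibility check, revealing its arrow.
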(event Custom|SetValues
  ;[1 1 1] Set up dynamic material instance (2)
  (for _array_element (Variables|Default|GetDynamicMaterials)
    (Rendering|Material|SetVectorParameterValue _array_element "Colour" (Variables|Default|GetColour) :!class /Script/Engine.MaterialInstanceDynamic)
    (Rendering|Material|SetScalarParameterValue _array_element "Metallic" (Variables|Default|GetMetallic) :!class /Script/Engine.MaterialInstanceDynamic)
    (Rendering|Material|SetScalarParameterValue _array_element "Roughness" (Variables|Default|GetRoughness) :!class /Script/Engine.MaterialInstanceDynamic)))

(event Custom|ExpandPlayer
  (params (Player :type BP%20Player%20Object%20Reference))
  ;[1 1 1] Attach coral to the player every time an enemy is eaten
  (AddComponent|AddStaticMeshComponent Player false (Math|Transform|MakeTransform "0, 0, 0" (Math|Rotator|MakeRotator (Math|Random|RandomFloatinRange 0.0 3.6e+02) (Math|Random|RandomFloatinRange 0.0 3.6e+02) (Math|Random|RandomFloatinRange 0.0 3.6e+02)) (Math|Conversions|ToVector(Float) (/ (Variables|Default|GetSize) (Utilities|Select :Index (Variables|Default|GetEnemyLevel) :Option%200 3.0 :Option%201 4.0 :Option%202 5.5 :Option%203 8.0 :Option%204 1e+01))))))

(event Custom|Restart
  ;[1 1 1] Wavy movement effect
  (bind _movement (Timeline|Timeline PlayFromStart)
    (:Update
      (Transformation|SetActorLocation (Math|Vector|Lerp(Vector) (Variables|Movement|GetStartLocation) (Variables|EndLocation|GetEndLocation) _movement) false false))
    (:Finished
      (CallFunction|Restart))))

(event Custom|OnCoralConsumedEvent
  ;[1 1 1] Visual cue if fodder can be consumed via event dispatch whenever a coral is eaten
  (if (<= (Variables|Default|GetSize) (Variables|/Game/Blueprints/BP_Player.BP_Player_C|GetPlayerSize (Variables|Default|GetPlayerRef)))
    (Rendering|SetVisibility (Variables|Default|GetArrow) true false)))

(event Custom|StopTimeline
  ;[1 1 1] Wavy movement effect
  (bind _movement (Timeline|Timeline Stop)
    (:Update
      (Transformation|SetActorLocation (Math|Vector|Lerp(Vector) (Variables|Movement|GetStartLocation) (Variables|EndLocation|GetEndLocation) _movement) false false))
    (:Finished
      (CallFunction|Restart))))

(event EventInteract
  (params (PlayerRef :type BP%20Player%20Object%20Reference))
  (bind _size (Variables|Default|GetSize))
  (bind _cameraboom (Variables|/Game/Blueprints/BP_Player.BP_Player_C|GetCameraBoom (Variables|Default|GetPlayerRef)))
  ;[1 1 1] Interface interaction that avoids referencing errors by handling the player variables inside the fodder area
  (if (> (Variables|/Game/Blueprints/BP_Player.BP_Player_C|GetPlayerSize PlayerRef) _size)
    (if (Variables|Default|GetIsEnemy)
      (Variables|/Game/Blueprints/BP_Player.BP_Player_C|SetHealth PlayerRef (- (Variables|/Game/Blueprints/BP_Player.BP_Player_C|GetHealth PlayerRef) 1e+01))
      (Audio|PlaySound2D "/Game/SFX/SFX_EnemyFodder.SFX_EnemyFodder" 1.0 1.0 0.0 0 0)
      (else
        (bind _output_get (Variables|/Game/Blueprints/BP_Player.BP_Player_C|SetPlayerSize PlayerRef (+ (/ _size 5e+01) (Variables|/Game/Blueprints/BP_Player.BP_Player_C|GetPlayerSize PlayerRef))))
        (Default|CallOnCoralConsumed (Variables|Default|GetPlayerRef))
        (CallFunction|ExpandPlayer PlayerRef)
        (Transformation|SetActorScale3D (Game|GetPlayerCharacter 0) (Math|Conversions|ToVector(Float) _output_get))
        (Variables|/Script/Engine.SpringArmComponent|SetTargetArmLength _cameraboom (+ (Variables|/Script/Engine.SpringArmComponent|GetTargetArmLength _cameraboom) (* _size 4.0)))
        (Audio|PlaySound2D "/Game/SFX/SFX_Fodder.SFX_Fodder" 1.0 1.0 0.0 0 0)))
    (CallFunction|StopTimeline)
    (Utilities|FlowControl|DelayUntilNextTick)
    (Actor|DestroyActor)))

(event EventBeginPlay
  (bind _returnvalue (Transformation|GetActorLocation))
  (bind _sphere (Variables|Default|GetSphere))
  ;[1 1 1] Level variable based on current level
  (Utilities|FlowControl|DelayUntilNextTick)
  (bind _asbp_player (Utilities|Casting|CastToBP_Player (Game|Player|GetPlayerPawn 0)))
  (Variables|Default|SetPlayerRef _asbp_player)
  (Variables|Default|SetEnemyLevel (Variables|/Game/Blueprints/BP_Player.BP_Player_C|GetCurrentLevel _asbp_player))
  (Rendering|SetVisibility (Variables|Default|GetArrow) false false)
  ;[1 1 1] Original dynamic material instance
  (for (_array_element _array_index) (Rendering|Material|GetMaterials _sphere)
    (bind _returnvalue_2 (Rendering|Material|CreateDynamicMaterialInstance _sphere _array_index _array_element "None" :!class /Script/Engine.PrimitiveComponent))
    (Utilities|Array|SetArrayElem (Variables|Default|GetDynamicMaterials) _array_index _returnvalue_2 true)
    (EventDispatchers|BindEventtoOnCoralConsumed (Variables|Default|GetPlayerRef) (delegate Custom|OnCoralConsumedEvent))
    ;[1 1 1] Set size to random float based on level
    (bind _output_get (Variables|Default|SetSize (Math|Random|RandomFloatinRange (Utilities|Select :Index (Variables|Default|GetEnemyLevel) :Option%200 0.25 :Option%201 0.5 :Option%202 1.0 :Option%203 1.5 :Option%204 2.5) (Utilities|Select :Index (Variables|Default|GetEnemyLevel) :Option%200 1.25 :Option%201 1.75 :Option%202 2.5 :Option%203 3.5 :Option%204 5.0))))
    (Transformation|SetActorScale3D (Math|Conversions|ToVector(Float) _output_get))
    ;[1 1 1] Call after setting all sizes
    (CallFunction|OnCoralConsumedEvent)
    ;[1 1 1] 1/10 chance for a fodder to be a static enemy
    (if (== (Math|Random|RandomIntegerinRange 1 10) 1)
      (Variables|Default|SetIsEnemy true)
      ;[1 1 1] Set colour based on enemy variable
      (Variables|Default|SetColour "(R=0.421875,G=0.000000,B=0.000000,A=1.000000)")
      (else
        (Variables|Default|SetIsEnemy false)
        (Variables|Default|SetColour "(R=0.000000,G=0.333333,B=0.036856,A=1.000000)")))
    (CallFunction|SetValues)
    ;[1 1 1] Wavy movement effect
    (Variables|Default|SetCustomTimeDilation (Math|Random|RandomFloatinRange 0.5 1.5))
    (Variables|Movement|SetStartLocation _returnvalue)
    (Variables|EndLocation|SetEndLocation (+ _returnvalue "0.000000,0.000000,25.000000"))
    (bind _movement (Timeline|Timeline Play)
      (:Update
        (Transformation|SetActorLocation (Math|Vector|Lerp(Vector) (Variables|Movement|GetStartLocation) (Variables|EndLocation|GetEndLocation) _movement) false false))
      (:Finished
        (CallFunction|Restart))))
  (CallFunction|SetValues))

(fn ConstructionScript)